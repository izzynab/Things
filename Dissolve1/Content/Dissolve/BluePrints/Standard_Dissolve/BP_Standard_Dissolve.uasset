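; Standard dissolve effect actor that animates a skeletal mesh's material alongside a Niagara effect when play begins.
; BeginPlay creates a dynamic material from slot 0 and passes a shared texture to both it and the Niagara component.
; A timeline then drives their "Amount" parameters together from a single interpolated value.
; When the timeline finishes, the Niagara "Width" is zeroed.
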(event `self.ReceiveBeginPlay`
  (bind _skeletalmesh (`self.SkeletalMesh`))
  (bind _niagara (`self.Niagara`))
  (bind _texture (`self.Texture`))
  (bind _returnvalue (`PrimitiveComponent.CreateDynamicMaterialInstance` _skeletalmesh 0 (`PrimitiveComponent.GetMaterial` _skeletalmesh 0) "None"))
  (`MaterialInstanceDynamic.SetTextureParameterValue` _returnvalue "Texture" _texture)
  (`NiagaraFunctionLibrary.SetTextureObject` (`self.Niagara`) "Texture" _texture)
  (bind (_direction _newtrack_0) (`Timeline|Timeline_0` :!via `PlayFromStart`)
    (:`Update`
      (`MaterialInstanceDynamic.SetScalarParameterValue` _returnvalue "Amount" (`KismetMathLibrary.Lerp` 1.0 0.0 _newtrack_0))
      (`NiagaraComponent.SetVariableFloat` _niagara "Amount" (`KismetMathLibrary.Lerp` 1.0 0.0 _newtrack_0)))
    (:`Finished`
      (`NiagaraComponent.SetVariableFloat` _niagara "Width" 0.0))))

(fn `UserConstructionScript`)