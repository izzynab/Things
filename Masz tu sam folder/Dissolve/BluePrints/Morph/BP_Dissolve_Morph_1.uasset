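; Blueprint that runs a particle dissolve morph from Character1 to Character2.
; After a short delay on BeginPlay, it attaches a Niagara system to Character1, feeds it both skeletal meshes, and animates MPC_Morph_D_1's Amount.
; The system exports particle data back to this Blueprint.
; When the first particle's Velocity-to-Position difference is small, a second timeline raises Amount1; otherwise that timeline is stopped, each once.
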(event `self.ReceiveBeginPlay`
  (bind _skeletalmeshcomponent (`SkeletalMeshActor.SkeletalMeshComponent` (`self.Character 1`)))
  (`KismetSystemLibrary.Delay` 1.0)
  (bind _returnvalue (`NiagaraFunctionLibrary.SpawnSystemAttached` (`self.niagara`) _skeletalmeshcomponent "None" (0.0 0.0 0.0) (struct) "KeepRelativeOffset"))
  (`NiagaraComponent.SetVariableObject` _returnvalue "CallBack" self)
  (`NiagaraFunctionLibrary.OverrideSystemUserVariableSkeletalMeshComponent` _returnvalue "Skeletal Mesh 1" _skeletalmeshcomponent)
  (`NiagaraFunctionLibrary.OverrideSystemUserVariableSkeletalMeshComponent` _returnvalue "Skeletal Mesh 2" (`SkeletalMeshActor.SkeletalMeshComponent` (`self.Character 2`)))
  (bind (_direction _newtrack_0) (`Timeline|Timeline_0` :!via `PlayFromStart`)
    (:`Update`
      (`KismetMaterialLibrary.SetScalarParameterValue` "/Game/Dissolve/Niagara_Dissolve/Morph_Effect/Morph_Dissolve_Effect/Const/MPC_Morph_D_1.MPC_Morph_D_1" "Amount" (`KismetMathLibrary.Lerp` 1.0 0.0 _newtrack_0)))))

(event `self.ReceiveParticleData`
  (params (Data :type "Array of BasicParticleData Structure (by ref)") (NiagaraSystem :type "NiagaraSystem Object Reference"))
  (bind (_position _size _velocity) (break `BasicParticleData` (`|GetArrayItem` Data)))
  (if (<= (`KismetMathLibrary.VSize` (- _velocity _position)) 80.0)
    (`/Engine/EditorBlueprintResources/StandardMacros.DoOnce` false
      (:`Completed`
        (bind (_direction _newtrack_0) (`Timeline|Timeline_2` :!via `PlayFromStart` :!label _label)
          (:`Update`
            (`KismetMaterialLibrary.SetScalarParameterValue` "/Game/Dissolve/Niagara_Dissolve/Morph_Effect/Morph_Dissolve_Effect/Const/MPC_Morph_D_1.MPC_Morph_D_1" "Amount1" (`KismetMathLibrary.Lerp` 0.0 1.0 _newtrack_0))))))
    (else
      (`/Engine/EditorBlueprintResources/StandardMacros.DoOnce` false
        (:`Completed`
          (goto _label :!via `Stop`))))))

(fn `UserConstructionScript`)