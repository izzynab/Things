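; BP_Morph_2 plays a dissolve-style morph effect between two referenced characters, Character1 and Character2, on BeginPlay.
; It attaches a Niagara system to Character1's mesh, feeds it both skeletal meshes and registers itself as the CallBack object.
; Two chained timelines, separated by a short delay, drive MPC_Morph_1: the first lowers Amount, then the second raises Amount1.
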(event `self.ReceiveBeginPlay`
  (bind _skeletalmeshcomponent (`SkeletalMeshActor.SkeletalMeshComponent` (`self.Character 1`)))
  (bind _returnvalue (`NiagaraFunctionLibrary.SpawnSystemAttached` (`self.niagara`) _skeletalmeshcomponent "None" (0.0 0.0 0.0) (struct) "KeepRelativeOffset"))
  (`NiagaraComponent.SetVariableObject` _returnvalue "CallBack" self)
  (`NiagaraFunctionLibrary.OverrideSystemUserVariableSkeletalMeshComponent` _returnvalue "Skeletal Mesh 1" _skeletalmeshcomponent)
  (`NiagaraFunctionLibrary.OverrideSystemUserVariableSkeletalMeshComponent` _returnvalue "Skeletal Mesh 2" (`SkeletalMeshActor.SkeletalMeshComponent` (`self.Character 2`)))
  (bind (_direction _newtrack_0) (`Timeline|Timeline_0` :!via `PlayFromStart`)
    (:`Update`
      (`KismetMaterialLibrary.SetScalarParameterValue` "/Game/Dissolve/Niagara_Dissolve/Morph_Effect/Morph_Effect/Const/MPC_Morph_1.MPC_Morph_1" "Amount" (`KismetMathLibrary.Lerp` 1.0 0.0 _newtrack_0)))
    (:`Finished`
      (`KismetSystemLibrary.Delay` 1.5)
      (bind (_direction_2 _newtrack_0_2) (`Timeline|Timeline_1` :!via `PlayFromStart`)
        (:`Update`
          (`KismetMaterialLibrary.SetScalarParameterValue` "/Game/Dissolve/Niagara_Dissolve/Morph_Effect/Morph_Effect/Const/MPC_Morph_1.MPC_Morph_1" "Amount1" (`KismetMathLibrary.Lerp` 0.0 1.0 _newtrack_0_2)))))))

(fn `UserConstructionScript`)