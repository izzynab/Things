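; Standard dissolve effect Blueprint for a static mesh, starting automatically on BeginPlay.
; It creates a dynamic material instance and passes the same texture to it and the Niagara system.
; A timeline drives the Amount parameter from 1 toward 0 on both material and particles in sync, then zeroes the Niagara Width when finished.
; A delay that would replay the effect is left unconnected.
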(event `self.ReceiveBeginPlay`
  (bind _static_mesh (`self.Static Mesh`))
  (bind _niagara (`self.Niagara`))
  (bind _texture (`self.Texture`))
  (bind _returnvalue (`PrimitiveComponent.CreateDynamicMaterialInstance` _static_mesh 0 (`PrimitiveComponent.GetMaterial` _static_mesh 0) "None"))
  (`MaterialInstanceDynamic.SetTextureParameterValue` _returnvalue "Texture" _texture)
  (`NiagaraFunctionLibrary.SetTextureObject` (`self.Niagara`) "Texture" _texture)
  (bind (_direction _newtrack_1) (`Timeline|Timeline_1`)
    (:`Update`
      (`MaterialInstanceDynamic.SetScalarParameterValue` _returnvalue "Amount" (`KismetMathLibrary.Lerp` 1.0 0.0 _newtrack_1))
      (`NiagaraComponent.SetVariableFloat` _niagara "Amount" (`KismetMathLibrary.Lerp` 1.0 0.0 _newtrack_1)))
    (:`Finished`
      (`NiagaraComponent.SetVariableFloat` _niagara "Width" 0.0))))

(fn `UserConstructionScript`)