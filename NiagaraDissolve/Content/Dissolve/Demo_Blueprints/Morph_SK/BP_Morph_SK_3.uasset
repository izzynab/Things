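; Demo Blueprint that morphs one skeletal mesh character into another through a particle-assisted dissolve.
; After a delay on BeginPlay, it attaches a Niagara system to the first character's mesh and binds both meshes as user variables.
; One timeline drives the first mesh's "Dissolve Amount" material parameter to dissolve it.
; A second timeline, triggered from the first's update through a delay, reverses that parameter on the second mesh to reveal it.
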(event `self.ReceiveBeginPlay`
  (bind _skeletalmeshcomponent (`SkeletalMeshActor.SkeletalMeshComponent` (`self.SK Character 1`)))
  (`KismetSystemLibrary.Delay` (`self.Delay`))
  (bind _returnvalue (`NiagaraFunctionLibrary.SpawnSystemAttached` (`self.niagara`) _skeletalmeshcomponent "None" (0.0 0.0 0.0) (struct) "KeepRelativeOffset"))
  (`NiagaraFunctionLibrary.OverrideSystemUserVariableSkeletalMeshComponent` _returnvalue "Skeletal Mesh 1" _skeletalmeshcomponent)
  (`NiagaraFunctionLibrary.OverrideSystemUserVariableSkeletalMeshComponent` _returnvalue "Skeletal Mesh 2" (`SkeletalMeshActor.SkeletalMeshComponent` (`self.SK Character 2`)))
  (bind (_direction _newtrack_0) (`Timeline|Timeline_0` :!via `PlayFromStart`)
    (:`Update`
      (`MeshComponent.SetScalarParameterValueOnMaterials` (`SkeletalMeshActor.SkeletalMeshComponent` (`self.SK Character 1`)) "Dissolve Amount" (`KismetMathLibrary.Lerp` -0.2 1.0 _newtrack_0))
      (`KismetSystemLibrary.Delay` 3.0)
      (bind (_direction_2 _newtrack_0_2) (`Timeline|Timeline_1`)
        (:`Update`
          (`MeshComponent.SetScalarParameterValueOnMaterials` (`SkeletalMeshActor.SkeletalMeshComponent` (`self.SK Character 2`)) "Dissolve Amount" (`KismetMathLibrary.Lerp` 1.0 -0.2 _newtrack_0_2)))))))

(fn `UserConstructionScript`)