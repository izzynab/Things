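; Demo Blueprint that morphs one static mesh into another using a dissolve effect and Niagara particles.
; After a configurable delay on BeginPlay, it spawns a Niagara system on the first mesh and feeds both meshes into its user variables.
; One timeline raises the first mesh's "Dissolve Amount" material parameter.
; Its updates trigger, through a further delay, a second timeline that lowers the parameter on the second mesh.
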(event `self.ReceiveBeginPlay`
  (bind _staticmeshcomponent (`StaticMeshActor.StaticMeshComponent` (`self.Static Mesh 1`)))
  (`KismetSystemLibrary.Delay` (`self.Delay`))
  (bind _returnvalue (`NiagaraFunctionLibrary.SpawnSystemAttached` (`self.niagara`) _staticmeshcomponent "None" (0.0 0.0 0.0) (struct) "KeepRelativeOffset"))
  (`NiagaraFunctionLibrary.OverrideSystemUserVariableStaticMeshComponent` _returnvalue "Static Mesh 1" _staticmeshcomponent)
  (`NiagaraFunctionLibrary.OverrideSystemUserVariableStaticMeshComponent` _returnvalue "Static Mesh 2" (`StaticMeshActor.StaticMeshComponent` (`self.Static Mesh 2`)))
  (bind (_direction _newtrack_0) (`Timeline|Timeline_0` :!via `PlayFromStart`)
    (:`Update`
      (`MeshComponent.SetScalarParameterValueOnMaterials` (`StaticMeshActor.StaticMeshComponent` (`self.Static Mesh 1`)) "Dissolve Amount" (`KismetMathLibrary.Lerp` -0.2 1.0 _newtrack_0))
      (`KismetSystemLibrary.Delay` 2.0)
      (bind (_direction_2 _newtrack_0_2) (`Timeline|Timeline_1`)
        (:`Update`
          (`MeshComponent.SetScalarParameterValueOnMaterials` (`StaticMeshActor.StaticMeshComponent` (`self.Static Mesh 2`)) "Dissolve Amount" (`KismetMathLibrary.Lerp` 1.0 -0.2 _newtrack_0_2)))))))

(fn `UserConstructionScript`)