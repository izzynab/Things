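; Blueprint that plays a timed skin dissolve effect on a referenced skeletal or static mesh character.
; After a BeginPlay delay, the StaticSkeletalMesh flag selects the skeletal (true) or static branch.
; Each branch creates a dynamic material on the first slot and spawns an attached Niagara system.
; A per-branch Timeline then drives "Dissolve Amount" down to zero, from a higher start for skeletal meshes.
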(event `self.ReceiveBeginPlay`
  (bind _skeletalmeshcomponent (`SkeletalMeshActor.SkeletalMeshComponent` (`self.Character (Skeletal)`)))
  (bind _staticmeshcomponent (`StaticMeshActor.StaticMeshComponent` (`self.Character (Static)`)))
  (`KismetSystemLibrary.Delay` (`self.Delay`))
  (if (`self.Static /Skeletal Mesh`)
    (bind _returnvalue (`PrimitiveComponent.CreateDynamicMaterialInstance` _skeletalmeshcomponent 0 null "None"))
    (`NiagaraFunctionLibrary.SpawnSystemAttached` (`self.niagara system`) _skeletalmeshcomponent "None" (0.0 0.0 0.0) (struct) "KeepRelativeOffset")
    (bind (_direction _newtrack_0) (`Timeline|Timeline` :!via `PlayFromStart`)
      (:`Update`
        (`MaterialInstanceDynamic.SetScalarParameterValue` _returnvalue "Dissolve Amount" (`KismetMathLibrary.Lerp` 2.0 0.0 _newtrack_0))))
    (else
      (bind _returnvalue_2 (`PrimitiveComponent.CreateDynamicMaterialInstance` _staticmeshcomponent 0 null "None"))
      (`NiagaraFunctionLibrary.SpawnSystemAttached` (`self.niagara system`) _staticmeshcomponent "None" (0.0 0.0 0.0) (struct) "KeepRelativeOffset")
      (bind (_direction_2 _newtrack_0_2) (`Timeline|Timeline_0` :!via `PlayFromStart`)
        (:`Update`
          (`MaterialInstanceDynamic.SetScalarParameterValue` _returnvalue_2 "Dissolve Amount" (`KismetMathLibrary.Lerp` 1.5 0.0 _newtrack_0_2)))))))

(fn `UserConstructionScript`)