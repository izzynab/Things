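; Static mesh actor Blueprint that adds and removes an outline by overlaying a second copy of its mesh with an outline material.
; The construction script assigns the mesh and can show an editor preview outline, which is destroyed on BeginPlay.
; At runtime, CreateOutline spawns the copy with dynamic material instances on the first or all slots, optionally on BeginPlay.
; DeleteOutline destroys that copy.
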(event `self.ReceiveBeginPlay`
  ;[1 1 1] Destroy outline preview on begin play
  (set `self.HasOultine` false)
  (`ActorComponent.K2_DestroyComponent` (`self.OutlinePreview`))
  (if (`self.ActivateOnBeginPlay`)
    (`self.Create Outline`)))

(event `Create Outline`
  ;[1 1 1] Create outline event
  (bind _returnvalue (`AddComponent|NODE_AddStaticMeshComponent-2` :`bManualAttachment` true :`RelativeTransform` (`SceneComponent.K2_GetComponentToWorld` (`self.Mesh`))))
  (bind _output_get (set `self.Outline Mesh` _returnvalue))
  (`StaticMeshComponent.SetStaticMesh` _output_get (`StaticMeshComponent.StaticMesh` (`self.Mesh`)))
  (if (`self.OutlineForAllMaterials`)
    (for _index (range (+ (`PrimitiveComponent.GetNumMaterials` (`self.Mesh`)) 1))
      (`PrimitiveComponent.CreateDynamicMaterialInstance` (`self.Outline Mesh`) _index (`self.Outline Material Instance`) "None"))
    (set `self.HasOultine` true)
    (else
      (`PrimitiveComponent.CreateDynamicMaterialInstance` (`self.Outline Mesh`) 0 (`self.Outline Material Instance`) "None")
      (set `self.HasOultine` true))))

(event `Delete Outline`
  ;[1 1 1] Delete outline event
  (`/Engine/EditorBlueprintResources/StandardMacros.IsValid` (`self.Outline Mesh`)
    (:`Is Valid`
      (`ActorComponent.K2_DestroyComponent` (`self.Outline Mesh`))
      (set `self.HasOultine` false))))

(fn `UserConstructionScript`
  ;[1 1 1] Mesh setup
  (`StaticMeshComponent.SetStaticMesh` (`self.Mesh`) (`self.StaticMesh`))
  ;[1 1 1] Outline preview setup
  (if (`self.EditorShowOutline`)
    (`StaticMeshComponent.SetStaticMesh` (`self.OutlinePreview`) (`self.StaticMesh`))
    (if (`self.OutlineForAllMaterials`)
      (for _index (range (+ (`PrimitiveComponent.GetNumMaterials` (`self.Mesh`)) 1))
        (`PrimitiveComponent.SetMaterial` (`self.OutlinePreview`) _index (`self.Outline Material Instance`)))
      (else
        (`PrimitiveComponent.SetMaterial` (`self.OutlinePreview`) 0 (`self.Outline Material Instance`))))))