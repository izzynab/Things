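; Blueprint for toggling an outline effect, named for use with skeletal meshes.
; On BeginPlay it sets the Outline component's visibility and the state flag HasOultine from ActivateOnBeginPlay.
; CreateOutline and DeleteOutline events show or hide that component without propagating to children, updating the flag to match.
; The construction script is empty, so the graphs only switch visibility and do no outline setup.
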(event `self.ReceiveBeginPlay`
  (bind _activateonbeginplay (`self.ActivateOnBeginPlay`))
  ;[1 1 1] Deactivate outline on begin play
  (set `self.HasOultine` _activateonbeginplay)
  (`SceneComponent.SetVisibility` (`self.Outline`) _activateonbeginplay false))

(event `Create Outline`
  ;[1 1 1] Activate outline
  (`SceneComponent.SetVisibility` (`self.Outline`) true false)
  (set `self.HasOultine` true))

(event `Delete Outline`
  ;[1 1 1] Deactivate outline
  (`SceneComponent.SetVisibility` (`self.Outline`) false false)
  (set `self.HasOultine` false))

(fn `UserConstructionScript`)