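; Body scan effect Blueprint that runs a looping scan line over a referenced static mesh actor using Niagara and materials.
; After a delay on BeginPlay, it attaches a Niagara system to the mesh component and feeds that mesh into the system's user variable.
; A self-restarting timeline drives the Niagara "Speed" and material "Line Speed" parameters with the same interpolated value, keeping both in sync.
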(event `self.ReceiveBeginPlay`
  (bind _staticmeshcomponent (`StaticMeshActor.StaticMeshComponent` (`self.Static Mesh`)))
  ;[1 1 1] Start
  (`KismetSystemLibrary.Delay` (`self.Delay`))
  ;[1 1 1] Setting up Niagara System
  (bind _returnvalue (`NiagaraFunctionLibrary.SpawnSystemAttached` (`self.Niagara System`) _staticmeshcomponent "None" (0.0 0.0 0.0) (struct) "KeepRelativeOffset"))
  (`NiagaraFunctionLibrary.OverrideSystemUserVariableStaticMeshComponent` _returnvalue "Static Mesh" _staticmeshcomponent)
  ;[1 1 1] Loop
  (bind (_direction _newtrack_0) (`Timeline|Timeline_0` :!via `PlayFromStart` :!label _label)
    (:`Update`
      (bind _returnvalue_2 (`KismetMathLibrary.Lerp` 0.15 1.15 _newtrack_0))
      ;[1 1 1] Setting up Niagara & Material float
      (`NiagaraComponent.SetVariableFloat` _returnvalue "Speed" _returnvalue_2)
      (`MeshComponent.SetScalarParameterValueOnMaterials` _staticmeshcomponent "Line Speed" _returnvalue_2))
    (:`Finished`
      (if true
        (goto _label :!via `PlayFromStart`)))))

(fn `UserConstructionScript`)