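; BP_Body_Scan_SK drives a looping body-scan line effect on a referenced skeletal mesh actor.
; On BeginPlay, after a delay, it attaches a Niagara system to the mesh component and feeds that component in as the system's skeletal mesh source.
; An endlessly restarting timeline lerps one value into both the Niagara "Speed" variable and the materials' "Line Speed" parameter, driving particles and shader together.
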(event `self.ReceiveBeginPlay`
  (bind _skeletalmeshcomponent (`SkeletalMeshActor.SkeletalMeshComponent` (`self.Skeletal Mesh`)))
  ;[1 1 1] Start
  (`KismetSystemLibrary.Delay` (`self.Delay`))
  ;[1 1 1] Setting up Niagara System
  (bind _returnvalue (`NiagaraFunctionLibrary.SpawnSystemAttached` (`self.Niagara System`) _skeletalmeshcomponent "None" (0.0 0.0 0.0) (struct) "KeepRelativeOffset"))
  (`NiagaraFunctionLibrary.OverrideSystemUserVariableSkeletalMeshComponent` _returnvalue "Skeletal Mesh" _skeletalmeshcomponent)
  ;[1 1 1] Loop
  (bind (_direction _newtrack_0) (`Timeline|Timeline_0` :!via `PlayFromStart` :!label _label)
    (:`Update`
      (bind _returnvalue_2 (`KismetMathLibrary.Lerp` 0.15 1.15 _newtrack_0))
      ;[1 1 1] Setting up Niagara & Material float
      (`NiagaraComponent.SetVariableFloat` _returnvalue "Speed" _returnvalue_2)
      (`MeshComponent.SetScalarParameterValueOnMaterials` _skeletalmeshcomponent "Line Speed" _returnvalue_2))
    (:`Finished`
      (if true
        (goto _label :!via `PlayFromStart`)))))

(fn `UserConstructionScript`)