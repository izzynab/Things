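; BP_Morph plays a Niagara particle morph from one skeletal mesh character to another.
; After a short delay it spawns NS_Morph on Character1, feeds it both meshes and animates MPC_Morph's Amount from 1 to 0.
; The system exports particle data back to the Blueprint, comparing one particle's Velocity and Position vectors.
; Once they are close, a one-shot timeline raises Amount1 from 0 to 1.
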(event `self.ReceiveBeginPlay`
  (bind _skeletalmeshcomponent (`SkeletalMeshActor.SkeletalMeshComponent` (`self.Character 1`)))
  (`KismetSystemLibrary.Delay` 3.0)
  (bind _returnvalue (`NiagaraFunctionLibrary.SpawnSystemAttached` "/Game/Dissolve/Niagara_Dissolve/Morph_Effect/NS_Morph.NS_Morph" _skeletalmeshcomponent "None" (0.0 0.0 0.0) (struct) "KeepRelativeOffset"))
  (`NiagaraComponent.SetVariableObject` _returnvalue "CallBack" self)
  (`NiagaraFunctionLibrary.OverrideSystemUserVariableSkeletalMeshComponent` _returnvalue "Skeletal Mesh 1" _skeletalmeshcomponent)
  (`NiagaraFunctionLibrary.OverrideSystemUserVariableSkeletalMeshComponent` _returnvalue "Skeletal Mesh 2" (`SkeletalMeshActor.SkeletalMeshComponent` (`self.Character 2`)))
  (bind (_direction _newtrack_0) (`Timeline|Timeline_0` :!via `PlayFromStart`)
    (:`Update`
      (`KismetMaterialLibrary.SetScalarParameterValue` "/Game/Dissolve/Niagara_Dissolve/Morph_Effect/Const/MPC_Morph.MPC_Morph" "Amount" (`KismetMathLibrary.Lerp` 1.0 0.0 _newtrack_0)))))

(event `self.ReceiveParticleData`
  (params (Data :type "Array of BasicParticleData Structure (by ref)") (NiagaraSystem :type "NiagaraSystem Object Reference"))
  (bind (_position _size _velocity) (break `BasicParticleData` (`|GetArrayItem` Data 1)))
  (if (<= (`KismetMathLibrary.VSize` (- _velocity _position)) 80.0)
    (`/Engine/EditorBlueprintResources/StandardMacros.DoOnce` false
      (:`Completed`
        (bind (_direction _newtrack_0) (`Timeline|Timeline_2` :!via `PlayFromStart`)
          (:`Update`
            (`KismetMaterialLibrary.SetScalarParameterValue` "/Game/Dissolve/Niagara_Dissolve/Morph_Effect/Const/MPC_Morph.MPC_Morph" "Amount1" (`KismetMathLibrary.Lerp` 0.0 1.0 _newtrack_0))))))))

(fn `UserConstructionScript`)